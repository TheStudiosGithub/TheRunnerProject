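; BP_CoinPickup is a collectible coin in TheRunner that the player picks up by running into it.
; On actor overlap with a ThirdPersonCharacter, it casts the game mode to ThirdPersonGameMode and increments both its Coins and Currency counters.
; It then destroys itself, so all coin totals live on the game mode rather than on the pickup or character.
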(event Collision|EventActorBeginOverlap
  (params (OtherActor :type Actor%20Object%20Reference))
  (Utilities|Casting|CastToThirdPersonCharacter OtherActor)
  (bind _asthird_person_game_mode (Utilities|Casting|CastToThirdPersonGameMode (Game|GetGameMode)))
  (Math|Integer|IncrementInt (Variables|/Game/TheRunner/BluePrints/ThirdPersonGameMode.ThirdPersonGameMode_C|GetCoins _asthird_person_game_mode)
    (:%20%20
      (bind _asthird_person_game_mode_2 (Utilities|Casting|CastToThirdPersonGameMode (Game|GetGameMode)))
      (Variables|/Game/TheRunner/BluePrints/ThirdPersonGameMode.ThirdPersonGameMode_C|SetCurrency _asthird_person_game_mode_2 (+ (Variables|/Game/TheRunner/BluePrints/ThirdPersonGameMode.ThirdPersonGameMode_C|GetCurrency _asthird_person_game_mode_2) 1))
      (Actor|DestroyActor))))

(fn ConstructionScript)