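; BP_FirstTile is a runner track tile that keeps the endless path going as the player crosses it.
; Overlapping NextSpawnTile makes ThirdPersonGameMode spawn a tile and add multiplied points, then rescales clamped walk speed (the 0.01 factor pins it to minimum) and destroys itself after a delay.
; SpawnObstacles, not called here, randomly places pipes, boxes or coins at three arrows in sequence, with a zero roll ending the chain.
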(event OnComponentBeginOverlap(NextSpawnTile)
  (params (OverlappedComponent :type Primitive%20Component%20Object%20Reference) (OtherActor :type Actor%20Object%20Reference) (OtherComp :type Primitive%20Component%20Object%20Reference) (OtherBodyIndex :type Integer) (bFromSweep :type Boolean) (SweepResult :type Hit%20Result%20Structure%20%28by%20ref%29))
  (Utilities|Casting|CastToThirdPersonCharacter OtherActor)
  (bind _asthird_person_game_mode (Utilities|Casting|CastToThirdPersonGameMode (Game|GetGameMode)))
  (Default|SpawnTile _asthird_person_game_mode)
  (bind _asthird_person_game_mode_2 (Utilities|Casting|CastToThirdPersonGameMode (Game|GetGameMode)))
  (bind _output_get (Variables|/Game/TheRunner/BluePrints/ThirdPersonGameMode.ThirdPersonGameMode_C|SetCurrentPoints _asthird_person_game_mode_2 (+ (* 1 (Variables|/Game/TheRunner/BluePrints/ThirdPersonGameMode.ThirdPersonGameMode_C|GetPointsMultiplier _asthird_person_game_mode_2)) (Variables|/Game/TheRunner/BluePrints/ThirdPersonGameMode.ThirdPersonGameMode_C|GetCurrentPoints _asthird_person_game_mode_2))))
  (Development|PrintString (Utilities|String|ToString(Integer) _output_get) false false)
  (bind _asthird_person_character (Utilities|Casting|CastToThirdPersonCharacter (Game|GetPlayerCharacter 0)))
  (Variables|/Script/Engine.CharacterMovementComponent|SetMaxWalkSpeed (Variables|/Script/Engine.Character|GetCharacterMovement _asthird_person_character) (Math|Float|Clamp(Float) (* (Variables|/Script/Engine.CharacterMovementComponent|GetMaxWalkSpeed (Variables|/Script/Engine.Character|GetCharacterMovement _asthird_person_character)) 0.01) 6e+02 1.2e+03))
  (Utilities|FlowControl|Delay 0.5)
  (Actor|DestroyActor))

(event EventBeginPlay)

(fn ConstructionScript)

(fn SpawnObstacles
  (bind _arrow (Variables|Default|GetArrow))
  (bind _arrow1 (Variables|Default|GetArrow1))
  (bind _arrow2 (Variables|Default|GetArrow2))
  (bind _returnvalue (Transformation|GetWorldTransform _arrow2))
  (bind _returnvalue_2 (Transformation|GetWorldTransform _arrow))
  (bind _returnvalue_3 (Transformation|GetWorldTransform _arrow1))
  (switch int (Math|Random|RandomIntegerinRange 0 3)
    (:1
      (Game|SpawnActorfromClass "/Game/TheRunner/MasterTile/Meshes/Obstacle_Pipe.Obstacle_Pipe_C" _returnvalue_2 "Undefined" 0 0))
    (:2
      (Game|SpawnActorfromClass "/Game/TheRunner/MasterTile/Meshes/Obstacle_Box.Obstacle_Box_C" _returnvalue_2 "Undefined" 0 0))
    (:3
      (Game|SpawnActorfromClass "/Game/TheRunner/BluePrints/BP_CoinPickup.BP_CoinPickup_C" _returnvalue_2 "Undefined" 0 0)))
  (switch int (Math|Random|RandomIntegerinRange 0 3)
    (:1
      (Game|SpawnActorfromClass "/Game/TheRunner/MasterTile/Meshes/Obstacle_Pipe.Obstacle_Pipe_C" _returnvalue_3 "Undefined" 0 0))
    (:2
      (Game|SpawnActorfromClass "/Game/TheRunner/MasterTile/Meshes/Obstacle_Box.Obstacle_Box_C" _returnvalue_3 "Undefined" 0 0))
    (:3
      (Game|SpawnActorfromClass "/Game/TheRunner/BluePrints/BP_CoinPickup.BP_CoinPickup_C" _returnvalue_3 "Undefined" 0 0)))
  (switch int (Math|Random|RandomIntegerinRange 0 3)
    (:1
      (Game|SpawnActorfromClass "/Game/TheRunner/MasterTile/Meshes/Obstacle_Pipe.Obstacle_Pipe_C" _returnvalue "Undefined" 0 0))
    (:2
      (Game|SpawnActorfromClass "/Game/TheRunner/MasterTile/Meshes/Obstacle_Box.Obstacle_Box_C" _returnvalue "Undefined" 0 0))
    (:3
      (Game|SpawnActorfromClass "/Game/TheRunner/BluePrints/BP_CoinPickup.BP_CoinPickup_C" _returnvalue "Undefined" 0 0))))